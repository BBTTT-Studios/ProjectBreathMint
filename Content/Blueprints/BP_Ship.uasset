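; Ship actor that is steered and propelled by a VR wheel lever and a VR slider.
; Every tick, the slider progress moves the ship along its right vector and the wheel's lever angle adds a scaled local yaw.
; Both steps are applied per frame without delta-time scaling or sweep.
; Two text components display the current wheel angle and slider progress.
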(event `self.ReceiveTick`
  (params (DeltaSeconds :type "Float (single-precision)"))
  (bind _currentleverangle (`VRLeverComponent.CurrentLeverAngle` (`self.Wheel`)))
  (bind _currentsliderprogress (`VRSliderComponent.CurrentSliderProgress` (`self.VRSlider`)))
  (`TextRenderComponent.K2_SetText` (`self.WheelText`) (`KismetTextLibrary.Conv_DoubleToText` _currentleverangle "HalfToEven"))
  (`self.K2_AddActorWorldOffset` (* (`self.GetActorRightVector`) (* _currentsliderprogress 4.0)))
  (`TextRenderComponent.K2_SetText` (`self.SliderText`) (`KismetTextLibrary.Conv_DoubleToText` _currentsliderprogress "HalfToEven"))
  (`self.K2_AddActorLocalRotation` (`KismetMathLibrary.MakeRotator` 0.0 0.0 (/ _currentleverangle 1000.0))))

(fn `UserConstructionScript`)