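; PlacingGun is a gun Blueprint that blows a bubble from its barrel while the trigger is held and launches it on release.
; Use spawns a tiny BP_Bubble at the barrel with physics off, and Tick grows and nudges it along the barrel's right vector each frame.
; UseStopped enables physics, clears velocity and applies a mass-independent impulse combining random scatter with a push along that vector.
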(event `/Game/Blueprints/I_Use.Use`
  (params (CallingController :type "GripMotionControllerComponent Object Reference"))
  (bind _barrelref (`self.BarrelRef`))
  (set `self.TriggerHeld` true)
  (bind _returnvalue (`|SpawnActorFromClass` "/Game/Blueprints/Guns/BP_Bubble.BP_Bubble_C" (`KismetMathLibrary.MakeTransform` (+ (`SceneComponent.K2_GetComponentLocation` _barrelref) (* (`SceneComponent.GetRightVector` _barrelref) 3.0)) (struct) (0.01 0.01 0.01)) "Undefined" "OverrideRootScale" null null))
  (`PrimitiveComponent.SetSimulatePhysics` (`/Game/Blueprints/Guns/BP_Bubble.BubbleMesh` _returnvalue) false)
  (set `self.CreatedActor` _returnvalue))

(event `/Game/Blueprints/I_Use.UseStopped`
  (bind _bubblemesh (`/Game/Blueprints/Guns/BP_Bubble.BubbleMesh` (`self.CreatedActor`)))
  (set `self.TriggerHeld` false)
  (`PrimitiveComponent.SetSimulatePhysics` _bubblemesh true)
  (`PrimitiveComponent.SetPhysicsLinearVelocity` _bubblemesh (0.0 0.0 0.0) false "None")
  (`PrimitiveComponent.AddImpulse` (`/Game/Blueprints/Guns/BP_Bubble.BubbleMesh` (`self.CreatedActor`)) (+ (* (`KismetMathLibrary.RandomUnitVector`) (`KismetMathLibrary.RandomFloatInRange` 20.0 40.0)) (* (`SceneComponent.GetRightVector` (`self.BarrelRef`)) 20.0)) "None" true))

(event `self.ReceiveTick`
  (params (DeltaSeconds :type "Float (single-precision)"))
  (bind _createdactor (`self.CreatedActor`))
  (if (`self.TriggerHeld`)
    (`/Engine/EditorBlueprintResources/StandardMacros.IsValid` _createdactor
      (:`Is Valid`
        (`self.SetActorScale3D` _createdactor (+ (`self.GetActorScale3D` (`self.CreatedActor`)) (0.01 0.01 0.01)))
        (`self.K2_AddActorLocalOffset` _createdactor (* (`SceneComponent.GetRightVector` (`self.BarrelRef`)) 2.0) false false)))))

(fn `UserConstructionScript`
  (`parent.UserConstructionScript`))