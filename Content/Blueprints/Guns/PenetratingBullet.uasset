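; PenetratingBullet is a projectile that simulates shooting through objects by respawning itself past what it hits.
; On a bounce with StrengthCoefficient below 0.9, it spawns a replacement at the computed exit, adds the coefficient to the impact velocity, and destroys itself.
; ComputeExitLocation sphere-traces backward from five units beyond the impact to find the exit.
; Only the first trace hit is checked, and the spawn ignores DidHit.
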(event `self.Projectile.OnProjectileBounce`
  (params (ImpactResult :type "HitResult Structure (by ref)") (ImpactVelocity :type "Vector Structure (by ref)"))
  (if (< (`self.StrengthCoefficient`) 0.9)
    (bind _exit_location (`self.ComputeExitLocation` ImpactResult ImpactVelocity))
    (bind _returnvalue (`|SpawnActorFromClass` "PenetratingBullet_C" (`KismetMathLibrary.MakeTransform` _exit_location) "Undefined" "OverrideRootScale" (`self.GetOwner`) null))
    (set `MovementComponent.Velocity` (+ ImpactVelocity (`self.StrengthCoefficient`)) (`/Game/Blueprints/Guns/BP_Bullet.Projectile` _returnvalue))
    (`self.K2_DestroyActor`)))

(fn `ComputeExitLocation`
  (params (Hit :type "HitResult Structure") (ImpactVelocity :type "Vector Structure"))
  (returns (`Exit Location` :type "Vector Structure") (DidHit :type Boolean))
  (bind (_bblockinghit _binitialoverlap _time _distance _location _impactpoint _normal _impactnormal _physmat _hitactor) (`GameplayStatics.BreakHitResult` Hit))
  (bind _outhits (`KismetSystemLibrary.SphereTraceMultiForObjects` (+ (* (`KismetMathLibrary.Normal` ImpactVelocity) 5) _location) _location (`SphereComponent.SphereRadius` (`self.CollisionComponent`)) (`|MakeArray` "ObjectTypeQuery1" "ObjectTypeQuery2" "ObjectTypeQuery3" "ObjectTypeQuery4" "ObjectTypeQuery5" "ObjectTypeQuery6" :!type "EObjectTypeQuery Enum")))
  (for _array_element _outhits
    (bind (_bblockinghit_2 _binitialoverlap_2 _time_2 _distance_2 _location_2 _impactpoint_2 _normal_2 _impactnormal_2 _physmat_2 _hitactor_2) (`GameplayStatics.BreakHitResult` _array_element))
    (if (== _hitactor_2 _hitactor)
      (return _location_2 true)
      (else
        (return (0.0 0.0 0.0) false)))))

(fn `UserConstructionScript`
  (`parent.UserConstructionScript`))