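; LaserGun is a grippable VR gun that fires an invisible line trace meant to bounce off surfaces, with no damage or effects yet.
; Gripping stores the controller and C_VREP holder, and Use triggers Shoot, which traces forward into Bounce.
; Bounce recurses when the hit material's Roughness is at least 0.1, squaring EnergyLeft.
; The reflection looks unfinished: its trace starts at the impact normal with no end set.
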(event `self.GrippableStaticMesh.OnGripped`
  (params (GrippingController :type "GripMotionControllerComponent Object Reference") (GripInformation :type "BPActorGripInformation Structure (by ref)"))
  (set `self.GrippingController` GrippingController)
  (bind _asc_vrep (cast `/Game/Blueprints/C_VREP` (`ActorComponent.GetOwner` GrippingController)))
  (set `self.HoldingCharacter` _asc_vrep)
  (set `self.ViewTicking` true))

(event `self.GrippableStaticMesh.OnDropped`
  (params (GrippingController :type "GripMotionControllerComponent Object Reference") (GripInformation :type "BPActorGripInformation Structure (by ref)") (bWasSocketed :type Boolean))
  (set `self.GrippingController` null)
  (set `self.HoldingCharacter` null)
  (set `self.ViewTicking` false))

(event `ShootGun`
  (set `self.IsFiring` true)
  (`self.Shoot` null))

(event `StopShooting`
  (set `self.IsFiring` false))

(event `/Game/Blueprints/I_Use.Use`
  (params (CallingController :type "GripMotionControllerComponent Object Reference"))
  (`self.ShootGun`))

(fn `Bounce`
  (params (Hit :type "HitResult Structure (by ref)"))
  (bind (_bblockinghit _binitialoverlap _time _distance _location _impactpoint _normal _impactnormal _physmat _hitactor _hitcomponent) (`GameplayStatics.BreakHitResult` Hit))
  (if (not (== _hitactor "/Game/Blueprints/C_VREP.C_VREP"))
    (bind _returnvalue (`PrimitiveComponent.CreateDynamicMaterialInstance` _hitcomponent 0 (`PrimitiveComponent.GetMaterial` _hitcomponent 0) "None"))
    (bind _output_get (set `self.ReflectedMat` _returnvalue))
    (bind _returnvalue_2 (`MaterialInstanceDynamic.K2_GetScalarParameterValue` _output_get "Roughness"))
    (if (>= _returnvalue_2 0.1)
      (set `self.EnergyLeft` (`KismetMathLibrary.Square` (`self.EnergyLeft`)))
      (bind _outhit (`KismetSystemLibrary.LineTraceSingleForObjects` _impactnormal (0.0 0.0 0.0) (`|MakeArray` "ObjectTypeQuery1" "ObjectTypeQuery2" "ObjectTypeQuery3" "ObjectTypeQuery4" "ObjectTypeQuery6" :!type "EObjectTypeQuery Enum")))
      (`self.Bounce` _outhit))))

(fn `Shoot`
  (params (Bullet :type "Actor Class Reference"))
  (bind _scene (`self.Scene`))
  (bind _returnvalue (`SceneComponent.K2_GetComponentLocation` _scene))
  (bind _outhit (`KismetSystemLibrary.LineTraceSingleForObjects` _returnvalue (+ _returnvalue (* (`SceneComponent.GetForwardVector` _scene) 5000)) (`|MakeArray` "ObjectTypeQuery1" "ObjectTypeQuery2" "ObjectTypeQuery3" "ObjectTypeQuery4" "ObjectTypeQuery6" :!type "EObjectTypeQuery Enum")))
  (`self.Bounce` _outhit))

(fn `UserConstructionScript`)