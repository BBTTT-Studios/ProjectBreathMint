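; Base VR gun Blueprint that tracks the gripping controller and its owning C_VREP character, toggling ViewTicking on grip and drop.
; Use triggers ShootGun, which sets IsFiring and calls Shoot to spawn a BP_BulletBase at the barrel with the mesh's rotation.
; Shoot then repeatedly sets that bullet's velocity to a fixed vector in a synchronous while loop on IsFiring, which StopShooting clears.
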(event `self.GrippableStaticMesh.OnGripped`
  (params (GrippingController :type "GripMotionControllerComponent Object Reference") (GripInformation :type "BPActorGripInformation Structure (by ref)"))
  (set `self.GrippingController` GrippingController)
  (bind _asc_vrep (cast `/Game/Blueprints/C_VREP` (`ActorComponent.GetOwner` GrippingController)))
  (set `self.HoldingCharacter` _asc_vrep)
  (set `self.ViewTicking` true))

(event `self.GrippableStaticMesh.OnDropped`
  (params (GrippingController :type "GripMotionControllerComponent Object Reference") (GripInformation :type "BPActorGripInformation Structure (by ref)") (bWasSocketed :type Boolean))
  (set `self.GrippingController` null)
  (set `self.HoldingCharacter` null)
  (set `self.ViewTicking` false))

(event `ShootGun`
  (set `self.IsFiring` true)
  (`self.Shoot`))

(event `StopShooting`
  (set `self.IsFiring` false))

(event `/Game/Blueprints/I_Use.Use`
  (params (CallingController :type "GripMotionControllerComponent Object Reference"))
  (`self.ShootGun`))

(fn `Shoot`
  (bind _returnvalue (`|SpawnActorFromClass` "/Game/Blueprints/Guns/BP_BulletBase.BP_BulletBase_C" (`KismetMathLibrary.MakeTransform` (`SceneComponent.K2_GetComponentLocation` (`self.BarrelRef`)) (`SceneComponent.K2_GetComponentRotation` (`self.GrippableStaticMesh`))) "Undefined" "OverrideRootScale" null null))
  (while (`self.IsFiring`)
    (`PrimitiveComponent.SetPhysicsLinearVelocity` (`/Game/Blueprints/Guns/BP_BulletBase.GrippableStaticMesh` _returnvalue) (10.0 10.0 10.0) false "None")))

(fn `UserConstructionScript`)