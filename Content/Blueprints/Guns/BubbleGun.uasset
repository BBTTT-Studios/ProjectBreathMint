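; A grippable bubble gun that emits particles while in use.
; Use and UseStopped set the Visible variable, whose RepNotify toggles the Small and Big emitters of its particle system, replicating the effect.
; Both emitters start disabled on BeginPlay, and dropping the gun disables them directly without changing Visible.
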(event `self.GrippableStaticMesh.OnDropped`
  (params (GrippingController :type "GripMotionControllerComponent Object Reference") (GripInformation :type "BPActorGripInformation Structure (by ref)") (bWasSocketed :type Boolean))
  (bind _particlesystem (`self.ParticleSystem`))
  (`FXSystemComponent.SetEmitterEnable` _particlesystem "Small" false)
  (`FXSystemComponent.SetEmitterEnable` _particlesystem "Big" false))

(event `self.ReceiveBeginPlay`
  (bind _particlesystem (`self.ParticleSystem`))
  (`SceneComponent.SetVisibility` _particlesystem true false)
  (`FXSystemComponent.SetEmitterEnable` _particlesystem "Small" false)
  (`FXSystemComponent.SetEmitterEnable` _particlesystem "Big" false))

(event `/Game/Blueprints/I_Use.Use`
  (params (CallingController :type "GripMotionControllerComponent Object Reference"))
  (set `self.Visible` true))

(event `/Game/Blueprints/I_Use.UseStopped`
  (set `self.Visible` false))

(fn `OnRep_Visible`
  (bind _visible (`self.Visible`))
  (bind _particlesystem (`self.ParticleSystem`))
  (`FXSystemComponent.SetEmitterEnable` _particlesystem "Small" _visible)
  (`FXSystemComponent.SetEmitterEnable` _particlesystem "Big" _visible))

(fn `UserConstructionScript`
  (`parent.UserConstructionScript`))