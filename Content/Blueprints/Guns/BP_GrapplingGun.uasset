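; VR grappling gun that pulls the holding C_VREP character toward surfaces whose components are tagged Grapple.
; Use sphere-traces from ShootSocket, spawns a BP_Hookpoint at the hit and attaches the visible cable to it.
; While connected, Tick applies spring-like pull with velocity damping to the character's VR movement; while held, it draws a debug aim line.
; Stopping use or dropping disconnects, but clears GrapplingActor before its destroy check, leaving hookpoints spawned.
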(event `/Game/Blueprints/I_Use.UseStopped`
  (bind _grapplingactor (`self.GrapplingActor`))
  (`SceneComponent.SetHiddenInGame` (`self.Cable`) true false)
  (set `self.GrappleConnected` false)
  (set `self.GrapplingActor` null)
  (`/Engine/EditorBlueprintResources/StandardMacros.IsValid` _grapplingactor
    (:`Is Valid`
      (`self.K2_DestroyActor` _grapplingactor))))

(event `/Game/Blueprints/I_Use.Use`
  (params (CallingController :type "GripMotionControllerComponent Object Reference"))
  (bind _grippablestaticmesh (`self.GrippableStaticMesh`))
  (bind _cable (`self.Cable`))
  (bind _returnvalue (`SceneComponent.GetSocketLocation` _grippablestaticmesh "ShootSocket"))
  (bind (_outhit _returnvalue_2) (`KismetSystemLibrary.SphereTraceSingle` _returnvalue (+ _returnvalue (* (`SceneComponent.GetRightVector` _grippablestaticmesh) (`self.HookDistance`))) 5.0 "TraceTypeQuery1" false (`|MakeArray` (`ActorComponent.GetOwner` CallingController))))
  (if _returnvalue_2
    (bind (_bblockinghit _binitialoverlap _time _distance _location _impactpoint _normal _impactnormal _physmat _hitactor _hitcomponent) (`GameplayStatics.BreakHitResult` _outhit))
    (if (`ActorComponent.ComponentHasTag` _hitcomponent "Grapple")
      (set `self.HookPoint` _impactpoint)
      (set `self.GrappleConnected` true)
      (`SceneComponent.SetHiddenInGame` _cable false false)
      (bind _returnvalue_3 (`|SpawnActorFromClass` "/Game/Blueprints/BP_Hookpoint.BP_Hookpoint_C" (`KismetMathLibrary.MakeTransform` (`self.HookPoint`)) "Undefined" "OverrideRootScale" null null))
      (bind _output_get (set `self.GrapplingActor` _returnvalue_3))
      (`CableComponent.SetAttachEndTo` _cable _output_get "None" "None"))))

(event `self.GrippableStaticMesh.OnGripped`
  (params (GrippingController :type "GripMotionControllerComponent Object Reference") (GripInformation :type "BPActorGripInformation Structure (by ref)"))
  (set `self.GrippingController` GrippingController)
  (bind _asc_vrep (cast `/Game/Blueprints/C_VREP` (`ActorComponent.GetOwner` GrippingController)))
  (set `self.HoldingCharacter` _asc_vrep)
  (set `self.ViewTicking` true))

(event `self.GrippableStaticMesh.OnDropped`
  (params (GrippingController :type "GripMotionControllerComponent Object Reference") (GripInformation :type "BPActorGripInformation Structure (by ref)") (bWasSocketed :type Boolean))
  (bind _grapplingactor (`self.GrapplingActor`))
  (set `self.GrippingController` null)
  (set `self.HoldingCharacter` null)
  (set `self.GrappleConnected` false)
  (set `self.GrapplingActor` null)
  (set `self.ViewTicking` false)
  (`/Engine/EditorBlueprintResources/StandardMacros.IsValid` _grapplingactor
    (:`Is Valid`
      (`self.K2_DestroyActor` _grapplingactor))))

(event `self.ReceiveTick`
  (params (DeltaSeconds :type "Float (single-precision)"))
  (bind _grippablestaticmesh (`self.GrippableStaticMesh`))
  (bind _returnvalue (`SceneComponent.GetSocketLocation` _grippablestaticmesh "ShootSocket"))
  (bind _vrmovementreference (`VRBaseCharacter.VRMovementReference` (`self.HoldingCharacter`)))
  (bind _returnvalue_2 (- (`SceneComponent.K2_GetComponentLocation` (`self.GrippableStaticMesh`)) (`self.HookPoint`)))
  (`|ExecutionSequence`
    (:`then_0`
      (if (`self.GrappleConnected`) :!label _label
        (`CharacterMovementComponent.AddForce` _vrmovementreference (* (* (`KismetMathLibrary.Normal` _returnvalue_2) (`KismetMathLibrary.Dot_VectorVector` _returnvalue_2 (`KismetMathLibrary.MakeVector` (.x (`self.GetVelocity` (`self.HoldingCharacter`))) (.y (`self.GetVelocity` (`self.HoldingCharacter`))) (* (.z (`self.GetVelocity` (`self.HoldingCharacter`))) 2.0)))) -2.0))
        (`CharacterMovementComponent.AddForce` _vrmovementreference (* (* (- (`SceneComponent.K2_GetComponentLocation` (`self.GrippableStaticMesh`)) (`self.HookPoint`)) 750.0) -1.0))))
    (:`then_1`
      (if (`self.ViewTicking`)
        (`|ExecutionSequence`
          (:`then_0`
            (`KismetSystemLibrary.LineTraceSingle` _returnvalue (+ _returnvalue (* (`SceneComponent.GetRightVector` _grippablestaticmesh) (`self.HookDistance`))) "TraceTypeQuery1" false (`|MakeArray` (`ActorComponent.GetOwner` (`self.GrippingController`))) "ForOneFrame")
            (goto _label))
          (:`then_1`
            (set `CableComponent.TileMaterial` (/ (`KismetMathLibrary.VSize` (- (`SceneComponent.GetSocketLocation` (`self.GrippableStaticMesh`) "ShootSocket") (`self.HookPoint`))) 100.0) (`self.Cable`))))))))

(fn `UserConstructionScript`)