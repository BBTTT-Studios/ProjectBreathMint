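; VREPPlayerController is a player controller that supplies motion controller thumbstick input as a 2D direction.
; GetJoystickDirection takes a left or right stick selection and returns that thumbstick's X and Y axis values as a vector, with Y inverted.
; The event graph and construction script contain no active logic.
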(fn `GetJoystickDirection`
  (params (Stick :type "/Game/GenericRadialMenus/UMG/EJoystickTypes Enum" :default "NewEnumerator0"))
  (returns (StickInput :type "Vector2D Structure"))
  (switch `/Game/GenericRadialMenus/UMG/EJoystickTypes` Stick
    (:`NewEnumerator0`
      (return (`KismetMathLibrary.MakeVector2D` (`self.GetInputAxisValue`) (* (`self.GetInputAxisValue`) -1.0))))
    (:`NewEnumerator1`
      (return (`KismetMathLibrary.MakeVector2D` (`self.GetInputAxisValue`) (* (`self.GetInputAxisValue`) -1.0))))))

(fn `UserConstructionScript`)