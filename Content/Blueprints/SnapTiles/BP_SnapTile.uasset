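; BP_SnapTile is a grippable tile with a text label that snaps onto a BP_TileReceptacle when dropped.
; Box overlap events track the current receptacle, counting only overlaps with that receptacle's Box component.
; On drop, the tile attaches to that receptacle if it has no tile, matching location and rotation, then shifts slightly upward.
; The label is set from TileText at construction and through RefreshText.
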(event `self.GrippableStaticMesh.OnDropped`
  (params (GrippingController :type "GripMotionControllerComponent Object Reference") (GripInformation :type "BPActorGripInformation Structure (by ref)") (bWasSocketed :type Boolean))
  (bind _overlappedreceptacle (`self.OverlappedReceptacle`))
  (`/Engine/EditorBlueprintResources/StandardMacros.IsValid` _overlappedreceptacle
    (:`Is Valid`
      (if (not (`/Game/Blueprints/SnapTiles/BP_TileReceptacle.HasTile` _overlappedreceptacle))
        (`self.K2_AttachToActor` (`self.OverlappedReceptacle`) "None" "SnapToTarget" "SnapToTarget" "KeepWorld")
        (`self.K2_AddActorWorldOffset` (0.0 0.0 3.0))))))

(event `RefreshText`
  (`TextRenderComponent.K2_SetText` (`self.text`) (`KismetTextLibrary.Conv_StringToText` (`self.TileText`))))

(event `self.Box.OnComponentBeginOverlap`
  (params (OverlappedComponent :type "PrimitiveComponent Object Reference") (OtherActor :type "Actor Object Reference") (OtherComp :type "PrimitiveComponent Object Reference") (OtherBodyIndex :type Integer) (bFromSweep :type Boolean) (SweepResult :type "HitResult Structure (by ref)"))
  (bind _asbp_tile_receptacle (cast `/Game/Blueprints/SnapTiles/BP_TileReceptacle` OtherActor))
  (if (== (`/Game/Blueprints/SnapTiles/BP_TileReceptacle.Box` _asbp_tile_receptacle) OtherComp)
    (set `self.OverlappedReceptacle` _asbp_tile_receptacle)))

(event `self.Box.OnComponentEndOverlap`
  (params (OverlappedComponent :type "PrimitiveComponent Object Reference") (OtherActor :type "Actor Object Reference") (OtherComp :type "PrimitiveComponent Object Reference") (OtherBodyIndex :type Integer))
  (bind _asbp_tile_receptacle (cast `/Game/Blueprints/SnapTiles/BP_TileReceptacle` OtherActor))
  (if (== (`/Game/Blueprints/SnapTiles/BP_TileReceptacle.Box` _asbp_tile_receptacle) OtherComp)
    (set `self.OverlappedReceptacle` null)))

(fn `UserConstructionScript`
  (`TextRenderComponent.K2_SetText` (`self.text`) (`KismetTextLibrary.Conv_StringToText` (`self.TileText`))))