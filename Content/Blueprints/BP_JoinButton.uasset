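; BP_JoinButton is a VR button actor meant for joining multiplayer games, with a text display for the server it finds.
; Five seconds after BeginPlay it runs a one-time Advanced Sessions search across all server types.
; The text shows the first result's server name, or "No Servers" if the search fails.
; The button's state-change handler only casts the game instance to ServerHostInstance, so no join is performed.
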(event `self.ReceiveBeginPlay`
  (`KismetSystemLibrary.K2_SetTimerDelegate` (delegate `FindSessions`) 5.0))

(event `FindSessions`
  (bind _results (`FindSessionsCallbackProxyAdvanced.FindSessionsAdvanced` (`GameplayStatics.GetPlayerController` 0) 0 false "AllServers")
    (:`OnSuccess`
      (bind _output_get (set `self.Session` (`|GetArrayItem` _results)))
      (`TextRenderComponent.K2_SetText` (`self.Text`) (`KismetTextLibrary.Conv_StringToText` (`FindSessionsCallbackProxy.GetServerName` _output_get))))
    (:`OnFailure`
      (`TextRenderComponent.K2_SetText` (`self.Text`) "No Servers"))))

(event `self.VRButton.OnButtonStateChanged`
  (params (ButtonState :type Boolean) (InteractingActor :type "Actor Object Reference") (InteractingComponent :type "PrimitiveComponent Object Reference"))
  (cast `/Game/Network/ServerHostInstance` (`GameplayStatics.GetGameInstance`)))

(fn `UserConstructionScript`)